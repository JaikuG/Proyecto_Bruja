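; BP_DamageGenerator applies periodic damage to the player while they are near its owner.
; Tick compares player-to-owner distance with DamageDistance, starting or clearing a looping one-second timer and printing Spanish debug messages.
; The timer calls CauseDamage, which passes DamageValue to the BP_Character's BPHealth.HealthUpdate.
; Each range branch sits behind a DoOnce with no visible reset, so each fires only once.
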(event `self.ReceiveTick`
  (params (DeltaSeconds :type "Float (single-precision)"))
  (if (< (`KismetMathLibrary.Vector_Distance` (`Actor.K2_GetActorLocation` (`self.GetOwner` self)) (`Actor.K2_GetActorLocation` (`GameplayStatics.GetPlayerPawn` 0))) (`self.DamageDistance`))
    (`/Engine/EditorBlueprintResources/StandardMacros.DoOnce` false
      (:`Completed`
        (`KismetSystemLibrary.PrintString` "Te hago daño :(")
        (`KismetSystemLibrary.K2_SetTimer` null "CauseDamage" 1.0 true)))
    (else
      (`/Engine/EditorBlueprintResources/StandardMacros.DoOnce` false
        (:`Completed`
          (`KismetSystemLibrary.PrintString` "No te hago daño :)")
          (`KismetSystemLibrary.K2_ClearTimer` null "CauseDamage"))))))

(fn `CauseDamage`
  (bind _asbp_character (cast `/Game/ProyectoBruja/Blueprints/BP_Character` (`GameplayStatics.GetPlayerCharacter` 0)))
  (`/Game/ProyectoBruja/Blueprints/BP_Health.HealthUpdate` (`/Game/ProyectoBruja/Blueprints/BP_Character.BP_Health` _asbp_character) (`self.DamageValue`)))
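; Inventory actor that can be opened as a container and also runs its own look-at detection to show an interaction prompt.
; On Tick it sphere-traces from the player camera, tracks the hit actor and sets a DisplayMessage widget to "Press E to Open" for any new hit, clearing it otherwise.
; Interactwith passes its BPInventorySystem to the player controller's HUD through ShowContainer.
; LookAt is a stub returning an empty string.
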(event `self.ReceiveBeginPlay`
  (bind _returnvalue (`|CreateWidget` "/Game/ProyectoBruja/Inventory/UI/UW_DisplayMessage.UW_DisplayMessage_C"))
  (bind _output_get (set `self.DisplayMessage` _returnvalue))
  (`UserWidget.AddToViewport` _output_get 0))

(event `self.ReceiveTick`
  (params (DeltaSeconds :type "Float (single-precision)"))
  (bind _returnvalue (`GameplayStatics.GetPlayerCameraManager` 0))
  (bind _returnvalue_2 (`self.K2_GetActorLocation` _returnvalue))
  (bind (_outhit _returnvalue_3) (`KismetSystemLibrary.SphereTraceSingle` :`Start` _returnvalue_2 :`End` (+ _returnvalue_2 (* (`self.GetActorForwardVector` _returnvalue) (`self.InteractionRange`))) :`Radius` 15.0 :`TraceChannel` "TraceTypeQuery3" :`bIgnoreSelf` false))
  (if _returnvalue_3
    (bind (_bblockinghit _binitialoverlap _time _distance _location _impactpoint _normal _impactnormal _physmat _hitactor) (`GameplayStatics.BreakHitResult` _outhit))
    (if (!= _hitactor (`self.LookAtActor`))
      (set `self.LookAtActor` _hitactor)
      (`/Game/ProyectoBruja/Inventory/UI/UW_DisplayMessage.ShowMessage` (`self.DisplayMessage`) "Press E to Open"))
    (else
      (set `self.LookAtActor` null)
      (`/Game/ProyectoBruja/Inventory/UI/UW_DisplayMessage.ShowMessage` (`self.DisplayMessage`) ""))))

(event `/Game/ProyectoBruja/Inventory/BPInterface_Interact.InteractWith`
  (params (PlayerCharacter :type "/Game/ProyectoBruja/Blueprints/BP_Character Object Reference"))
  (bind _asbp_player_controller (cast `/Game/ProyectoBruja/Blueprints/BP_PlayerController` (`GameplayStatics.GetPlayerController` 0)))
  (`/Game/ProyectoBruja/Blueprints/UW_PlayerHUD.ShowContainer` (`/Game/ProyectoBruja/Blueprints/BP_PlayerController.HUD` _asbp_player_controller) (`self.BP_InventorySystem`)))

(fn `LookAt`
  (returns (Message :type Text))
  (return ""))

(fn `UserConstructionScript`)
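; BP_GateRight is a gate actor, named as the right-hand one, that swings open when asked while the player is nearby.
; Its OpenGate event receives the player's location and checks the horizontal distance to the gate against a fixed threshold, printing debug messages.
; Within range, it plays the gate sound and runs the DoorOpening timeline, which scales the Angle variable to set the static mesh's relative yaw.
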(event `/Game/ProyectoBruja/Inventory/BPInterface_Gate.OpenGate`
  (params (PlayerLocation :type "Vector Structure"))
  (bind (_returnvalue_x _returnvalue_y) (`KismetMathLibrary.BreakVector` (`self.K2_GetActorLocation`)))
  (bind _returnvalue (`KismetMathLibrary.Vector_Distance` (`KismetMathLibrary.MakeVector` PlayerLocation_X PlayerLocation_Y) (`KismetMathLibrary.MakeVector` _returnvalue_x _returnvalue_y)))
  (`KismetSystemLibrary.PrintString` (`KismetStringLibrary.Conv_DoubleToString` _returnvalue))
  (if (< _returnvalue 500.0)
    (`KismetSystemLibrary.PrintString` "Me abro")
    (`GameplayStatics.PlaySoundAtLocation` "/Game/ProyectoBruja/Assets/Sounds/S_Gate.S_Gate" (`self.K2_GetActorLocation`) (struct) 1.0 1.0 0.0 null null null null)
    (bind (_direction _newtrack_0) (`Timeline|doorOpening`)
      (:`Update`
        (`SceneComponent.K2_SetRelativeRotation` (`self.StaticMesh`) (`KismetMathLibrary.MakeRotator` 0.0 0.0 (* _newtrack_0 (`self.Angle`))) false false)))))

(fn `UserConstructionScript`)